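; BP_Elevator is an interactable elevator, labeled "Ride Elevator" for look-at, that moves its Cube vertically.
; Interactwith plays the ElevatorPosition timeline unless IsElevating is set, scaling its output into the Cube's relative height.
; The timeline's Finished output calls ElevatorDown to reverse it and clears IsElevating, which each update sets.
; Trigger's OnTriggered calls ElevatorUp, which is empty, or ElevatorDown when untriggered.
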(event `/Game/BPI_Interactable.InteractWith`
  (params (Player :type "/Game/FirstPerson/Blueprints/BP_FirstPersonCharacter Object Reference"))
  (if (not (`self.IsElevating`))
    (bind (_direction _position) (`Timeline|ElevatorPosition` :!label _label)
      (:`Update`
        (`SceneComponent.K2_SetRelativeLocation` (`self.Cube`) (* (0.0 0.0 250.0) _position) false false)
        (set `self.IsElevating` true))
      (:`Finished`
        (`self.ElevatorDown`)
        (set `self.IsElevating` false)))))

(event `ElevatorUp`)

(event `ElevatorDown`
  (goto _label :!via `Reverse`))

(event `self.Trigger.OnTriggered`
  (params (IsTriggered :type Boolean))
  (if IsTriggered
    (`self.ElevatorUp`)
    (else
      (`self.ElevatorDown`))))

(fn `LookAt`
  (returns (Verb :type Text) (Noun :type Text))
  (return "Ride" "Elevator"))

(fn `UserConstructionScript`)