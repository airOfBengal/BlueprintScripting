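; A rotating door that opens on interaction when unlocked and closes when the player leaves its overlap area.
; The DoorOpening timeline yaws DoorBase up to 90 degrees and plays in reverse to close.
; A linked Switch's trigger event locks or unlocks it, with a point light showing red or green, also set at construction.
; LookAt supplies the "Open Door" prompt text.
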(event `self.ReceiveActorBeginOverlap`
  (params (OtherActor :type "Actor Object Reference"))
  (if (== OtherActor (`GameplayStatics.GetPlayerCharacter` 0))
    _))

(event `self.ReceiveActorEndOverlap`
  (params (OtherActor :type "Actor Object Reference"))
  (if (== (`GameplayStatics.GetPlayerCharacter` 0) OtherActor)
    (`self.CloseDoor`)))

(event `OpenDoor`
  (if (not (`self.IsLocked`))
    (bind (_direction _rotation) (`Timeline|DoorOpening` :!label _label)
      (:`Update`
        (`SceneComponent.K2_SetRelativeRotation` (`self.DoorBase`) (* (struct :`Yaw` 90.0) _rotation) false false)))))

(event `CloseDoor`
  (goto _label :!via `Reverse`))

(event `self.Switch.OnSwitchTriggered`
  (params (IsTriggered :type Boolean))
  (if IsTriggered
    (`self.UnlockDoor`)
    (else
      (`self.LockDoor`))))

(event `/Game/BPI_Interactable.InteractWith`
  (params (Player :type "/Game/FirstPerson/Blueprints/BP_FirstPersonCharacter Object Reference"))
  (`self.OpenDoor`))

(fn `LockDoor`
  (bind _output_get (set `self.IsLocked` true))
  (`self.UpdateLockColor` _output_get))

(fn `LookAt`
  (returns (Verb :type Text) (Noun :type Text))
  (return "Open" "Door"))

(fn `UnlockDoor`
  (bind _output_get (set `self.IsLocked` false))
  (`self.UpdateLockColor` _output_get))

(fn `UpdateLockColor`
  (params (bIsLocked :type Boolean))
  (`LightComponent.SetLightColor` (`self.PointLight`) (`KismetMathLibrary.SelectColor` (struct :`R` 1.0 :`A` 1.0) (struct :`G` 1.0 :`A` 1.0) bIsLocked) true))

(fn `UserConstructionScript`
  (`self.UpdateLockColor` (`self.IsLocked`)))