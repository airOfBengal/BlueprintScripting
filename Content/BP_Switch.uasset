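; Player-activated switch that signals a triggered state for a limited time.
; Player overlap fires the OnSwitchTriggered dispatcher with true and sets a timer for UnlockDuration.
; If IsSwitchOff, a timeline lowers the handle; on expiry the timer broadcasts false and reverses the timeline.
; SwitchOn and SwitchOff only set that flag, which gates the animation but not the broadcast.
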(event `self.ReceiveActorBeginOverlap`
  (params (OtherActor :type "Actor Object Reference"))
  (if (== OtherActor (`GameplayStatics.GetPlayerCharacter` 0))
    (`self.SwitchTriggered`)))

(event `self.ReceiveActorEndOverlap`
  (params (OtherActor :type "Actor Object Reference"))
  (if (== OtherActor (`GameplayStatics.GetPlayerCharacter` 0))
    _))

(event `SwitchTriggered`
  (`self.OnSwitchTriggered` true)
  (`KismetSystemLibrary.K2_SetTimerDelegate` (delegate `SwitchUntriggered`) (`self.UnlockDuration`))
  (if (`self.IsSwitchOff`)
    (bind (_direction _position) (`Timeline|SwitchTriggering` :!label _label)
      (:`Update`
        (`SceneComponent.K2_SetRelativeLocation` (`self.SwitchHandle`) (* (62.5 0.0 -60.0) (`KismetMathLibrary.MakeVector` 1.0 0.0 _position)) false false)))))

(event `SwitchUntriggered`
  (`self.OnSwitchTriggered` false)
  (goto _label :!via `Reverse`))

(fn `SwitchOff`
  (set `self.IsSwitchOff` true))

(fn `SwitchOn`
  (set `self.IsSwitchOff` false))

(fn `UserConstructionScript`)