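; BP_Button is an interactable push button that shows "Push" and "Button" as its look-at verb and noun.
; Interacting fires OnTriggered with true, shifts the Cube to a pressed position and starts a timer of TimeoutTime.
; OnButtonTriggered, the apparent timer callback, returns the Cube to rest and fires OnTriggered with false, making the press momentary.
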(event `/Game/BPI_Interactable.InteractWith`
  (params (Player :type "/Game/FirstPerson/Blueprints/BP_FirstPersonCharacter Object Reference"))
  (`self.OnTriggered` true)
  (`SceneComponent.K2_SetRelativeLocation` (`self.Cube`) (-10.0 0.0 0.0) false false)
  (`KismetSystemLibrary.K2_SetTimerDelegate` (`|CreateDelegate` :!event `OnButtonTriggered`) (`self.TimeoutTime`)))

(fn `LookAt`
  (returns (Verb :type Text) (Noun :type Text))
  (return "Push" "Button"))

(fn `OnButtonTriggered`
  (`SceneComponent.K2_SetRelativeLocation` (`self.Cube`) (0.0 0.0 0.0) false false)
  (`self.OnTriggered` false))

(fn `UserConstructionScript`
  (`parent.UserConstructionScript`))