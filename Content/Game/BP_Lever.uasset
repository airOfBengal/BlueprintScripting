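; BP_Lever is an interactable lever that shows a "Pull Lever" prompt and toggles between pulled and released.
; Interacting plays or reverses the Rotation timeline based on IsPulled, lerping the Scene component through a 90-degree relative rotation.
; When the timeline finishes, its direction sets IsPulled and is broadcast through OnTriggered, so the state changes only once the movement completes.
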(event `/Game/BPI_Interactable.InteractWith`
  (params (Player :type "/Game/FirstPerson/Blueprints/BP_FirstPersonCharacter Object Reference"))
  (if (`self.IsPulled`)
    (bind (_direction _rotation) (`Timeline|Rotation` :!via `Reverse` :!label _label)
      (:`Update`
        (`SceneComponent.K2_SetRelativeRotation` (`self.Scene`) (`KismetMathLibrary.RLerp` (struct) (struct :`Pitch` 90.0) _rotation) false false))
      (:`Finished`
        (bind _returnvalue (select `ETimelineDirection` _direction :`Forward` true))
        (`self.OnTriggered` _returnvalue)
        (set `self.IsPulled` _returnvalue)))
    (else
      (goto _label))))

(fn `LookAt`
  (returns (Verb :type Text) (Noun :type Text))
  (return "Pull" "Lever"))

(fn `UserConstructionScript`
  (`parent.UserConstructionScript`))