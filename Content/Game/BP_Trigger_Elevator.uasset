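; BP_Trigger_Elevator is an interactable elevator trigger that moves its cube up and down, showing a "Move Elevator" prompt through LookAt.
; Interacting plays or reverses the Position timeline based on IsActive, scaling its output by UpDistance to set the cube's relative height.
; When the timeline finishes, its direction sets IsActive and is broadcast through OnTriggered, true for up and false for down.
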(event `/Game/BPI_Interactable.InteractWith`
  (params (Player :type "/Game/FirstPerson/Blueprints/BP_FirstPersonCharacter Object Reference"))
  (if (`self.IsActive`)
    (bind (_direction _position) (`Timeline|Position` :!via `Reverse` :!label _label)
      (:`Update`
        (`SceneComponent.K2_SetRelativeLocation` (`self.Cube`) (* _position (`KismetMathLibrary.MakeVector` 0.0 0.0 (`self.UpDistance`))) false false))
      (:`Finished`
        (bind _returnvalue (select `ETimelineDirection` _direction :`Forward` true))
        (`self.OnTriggered` _returnvalue)
        (set `self.IsActive` _returnvalue)))
    (else
      (goto _label))))

(fn `LookAt`
  (returns (Verb :type Text) (Noun :type Text))
  (return "Move" "Elevator"))

(fn `UserConstructionScript`
  (`parent.UserConstructionScript`))