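; BP_Pickup is a world item pickup that a player can interact with to add it to their inventory.
; A data asset defines the item, and the construction script applies its static mesh when the asset is valid.
; LookAt returns a "Pickup" verb and the item's name.
; Interactwith passes the asset and quantity to the player's InventorySystem and destroys the actor only if the add succeeds.
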(event `/Game/BPI_Interactable.InteractWith`
  (params (Player :type "/Game/FirstPerson/Blueprints/BP_FirstPersonCharacter Object Reference"))
  (bind _return (`/Game/Game/InventorySystem/InventorySystem.AddToInventory` (`/Game/FirstPerson/Blueprints/BP_FirstPersonCharacter.InventorySystem` Player) (`self.DataAsset`) (`self.Quantity`)))
  (if _return
    (`self.K2_DestroyActor`)))

(fn `LookAt`
  (returns (Verb :type Text) (Noun :type Text))
  (return "Pickup" (`/Game/Game/InventorySystem/Data/DA_Item.Name` (`self.DataAsset`))))

(fn `UserConstructionScript`
  (bind _dataasset (`self.DataAsset`)
    (:`then`
      (`StaticMeshComponent.SetStaticMesh` (`self.StaticMesh`) (`/Game/Game/InventorySystem/Data/DA_Item.StaticMesh` _dataasset)))
    (:`else`)))